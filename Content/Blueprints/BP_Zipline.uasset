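; BP_Zipline is a placeable zipline that carries the player one way from a positive-ID endpoint to its negative-ID partner.
; On BeginPlay the positive end finds its partner, stretches and rotates a cylinder mesh as the cable, and sets the Timeline play rate from distance and Time.
; A box overlap registers the zipline on the character.
; The Zipline event locks movement and lerps player 0 along the line until the Timeline finishes.
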(event OnComponentBeginOverlap(Box)
  (params (OverlappedComponent :type Primitive%20Component%20Object%20Reference) (OtherActor :type Actor%20Object%20Reference) (OtherComp :type Primitive%20Component%20Object%20Reference) (OtherBodyIndex :type Integer) (bFromSweep :type Boolean) (SweepResult :type Hit%20Result%20Structure%20%28by%20ref%29))
  (bind _asbp_third_person_character (Utilities|Casting|CastToBP_ThirdPersonCharacter OtherActor))
  (Variables|Default|SetPlayer _asbp_third_person_character)
  (Variables|/Game/ThirdPerson/Blueprints/BP_ThirdPersonCharacter.BP_ThirdPersonCharacter_C|SetbInZiplineZone (Variables|Default|GetPlayer) true)
  (Variables|/Game/ThirdPerson/Blueprints/BP_ThirdPersonCharacter.BP_ThirdPersonCharacter_C|SetZipline (Variables|Default|GetPlayer) self))

(event OnComponentEndOverlap(Box)
  (params (OverlappedComponent :type Primitive%20Component%20Object%20Reference) (OtherActor :type Actor%20Object%20Reference) (OtherComp :type Primitive%20Component%20Object%20Reference) (OtherBodyIndex :type Integer))
  (bind _player (Variables|Default|GetPlayer))
  (Variables|/Game/ThirdPerson/Blueprints/BP_ThirdPersonCharacter.BP_ThirdPersonCharacter_C|SetbInZiplineZone _player false)
  (Variables|/Game/ThirdPerson/Blueprints/BP_ThirdPersonCharacter.BP_ThirdPersonCharacter_C|SetZipline _player 0))

(event Custom|Zipline
  (bind _player (Variables|Default|GetPlayer))
  (if (Variables|/Game/ThirdPerson/Blueprints/BP_ThirdPersonCharacter.BP_ThirdPersonCharacter_C|GetbCanMove _player)
    (if (> (Variables|Default|GetID) 0)
      (if (not (Variables|/Game/ThirdPerson/Blueprints/BP_ThirdPersonCharacter.BP_ThirdPersonCharacter_C|GetbIsOnZipline _player))
        (Variables|/Game/ThirdPerson/Blueprints/BP_ThirdPersonCharacter.BP_ThirdPersonCharacter_C|SetbIsOnZipline _player true)
        (Variables|/Game/ThirdPerson/Blueprints/BP_ThirdPersonCharacter.BP_ThirdPersonCharacter_C|SetbCanMove _player false)
        (bind _newtrack_0 (Timeline|Timeline PlayFromStart)
          (:Update
            (Transformation|SetActorLocation (Game|GetPlayerCharacter 0) (Math|Vector|Lerp(Vector) (+ (Transformation|GetActorLocation) "0.000000,0.000000,60.000000") (+ (Variables|Default|GetLocationToGo) "0.000000,0.000000,60.000000") _newtrack_0) false false))
          (:Finished
            (Variables|/Game/ThirdPerson/Blueprints/BP_ThirdPersonCharacter.BP_ThirdPersonCharacter_C|SetbIsOnZipline _player false)
            (Variables|/Game/ThirdPerson/Blueprints/BP_ThirdPersonCharacter.BP_ThirdPersonCharacter_C|SetbCanMove _player true)))))))

(event EventBeginPlay
  (bind _returnvalue (Transformation|GetActorLocation))
  (bind _staticmesh (Variables|Default|GetStaticMesh))
  (if (> (Variables|Default|GetID) 0)
    (bind _outactors (Actor|GetAllActorsOfClass "BP_Zipline_C"))
    (for _array_element _outactors
      (if (== (Variables|BP_Zipline_C|GetID _array_element) (* (Variables|Default|GetID) -1))
        (bind _output_get (Variables|Default|SetLocationToGo (Transformation|GetActorLocation _array_element)))
        (Variables|Default|SetSpeed (/ (Math|Float|Sqrt (+ (+ (Math|Float|Square (- (.x _returnvalue) (.x _output_get))) (Math|Float|Square (- (.y _returnvalue) (.y _output_get)))) (Math|Float|Square (- (.z _returnvalue) (.z _output_get))))) 3.0))
        (Components|StaticMesh|SetStaticMesh _staticmesh "/Game/LevelPrototyping/Meshes/SM_Cylinder.SM_Cylinder")
        (Rendering|Material|SetMaterial _staticmesh 0 "/Game/LevelPrototyping/Materials/MM_Zipline.MM_Zipline")
        (Transformation|SetRelativeScale3D _staticmesh (Math|Vector|MakeVector 0.2 0.2 (/ (Math|Float|Sqrt (+ (+ (Math|Float|Square (- (.x _returnvalue) (.x _output_get))) (Math|Float|Square (- (.y _returnvalue) (.y _output_get)))) (Math|Float|Square (- (.z _returnvalue) (.z _output_get))))) 1.1e+02)))
        (Transformation|SetRelativeRotation _staticmesh (Math|Rotator|FindLookatRotation (+ (Variables|/Script/Engine.SceneComponent|GetRelativeLocation (Variables|Default|GetZipline_Position)) (Math|Vector|MakeVector (.x _returnvalue) (.y _returnvalue) (.z _returnvalue))) (+ (Transformation|GetActorLocation _array_element) (Variables|/Script/Engine.SceneComponent|GetRelativeLocation (Variables|BP_Zipline_C|GetZipline_Position _array_element)))) false false)
        (Transformation|AddRelativeRotation _staticmesh "-90.000000,0.000000,0.000000" false false)
        (Components|Timeline|SetPlayRate (Variables|Default|GetTimeline) (/ (/ (Variables|Default|GetSpeed) 1e+02) (Variables|Default|GetTime)))))))

(event Collision|EventActorBeginOverlap
  (params (OtherActor :type Actor%20Object%20Reference)))

(event EventTick
  (params (DeltaSeconds :type Float%20%28single-precision%29)))

(fn ConstructionScript)